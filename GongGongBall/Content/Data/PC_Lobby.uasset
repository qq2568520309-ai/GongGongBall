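; Lobby player controller that creates the lobby UI for the local player and registers their name from the game instance.
; ServerAddNewPlayer writes the name to PS_Lobby and calls its UpdatePlayer.
; UpdatePlayerInfos rebuilds the widget's player list from the names it receives, one UMG_PlayerInfo per entry.
; An authority check disables the Enter Game button on remote clients, leaving it to the host.
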(event `self.ReceiveBeginPlay`
  (if (`self.IsLocalPlayerController`)
    (set `self.bShowMouseCursor` true)
    (bind _returnvalue (`|CreateWidget` "/Game/UI/UMG_Lobby.UMG_Lobby_C"))
    (`UserWidget.AddToViewport` _returnvalue 0)
    (set `self.UMG_Lobby` _returnvalue)
    (`self.ServerAddNewPlayer` (`/Game/Data/GI_Main.PlayerName` (cast `/Game/Data/GI_Main` (`GameplayStatics.GetGameInstance`) :!pure true)))
    (`/Engine/EditorBlueprintResources/ActorMacros.Switch Has Authority`
      (:`Remote`
        (`Widget.SetIsEnabled` (`/Game/UI/UMG_Lobby.BTN_EnterGame` (`self.UMG_Lobby`)) false)))))

(event `UpdatePlayerInfos`
  (params (NewParam :type "Array of Text"))
  (bind _players (`/Game/UI/UMG_Lobby.Players` (`self.UMG_Lobby`)))
  (`PanelWidget.ClearChildren` _players)
  (for _array_element NewParam
    (bind _returnvalue (`|CreateWidget` "/Game/UI/UMG_PlayerInfo.UMG_PlayerInfo_C"))
    (`PanelWidget.AddChild` _players _returnvalue)
    (`TextBlock.SetText` (`/Game/UI/UMG_PlayerInfo.Name` _returnvalue) _array_element)))

(event `ServerAddNewPlayer`
  (params (NewParam :type Text))
  (bind _asps_lobby (cast `/Game/Data/PS_Lobby` (`self.PlayerState`)))
  (set `/Game/Data/PS_Lobby.PlayerNameInfo` NewParam _asps_lobby)
  (`/Game/Data/PS_Lobby.UpdatePlayer` _asps_lobby))

(fn `UserConstructionScript`)