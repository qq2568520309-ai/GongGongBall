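; BP_Bound is a boundary actor that detects when a BP_IceBall crosses its plane and reports the losing player.
; On the server, an ice ball overlap on a WinBound-type boundary prints an on-screen message that the player with this bound's PlayerIndex lost; no further game logic follows.
; The construction script gives the plane a dynamic M_Transparent material instance with its Debug parameter switched on.
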(event `self.Plane.OnComponentBeginOverlap`
  (params (OverlappedComponent :type "PrimitiveComponent Object Reference") (OtherActor :type "Actor Object Reference") (OtherComp :type "PrimitiveComponent Object Reference") (OtherBodyIndex :type Integer) (bFromSweep :type Boolean) (SweepResult :type "HitResult Structure (by ref)"))
  (`/Engine/EditorBlueprintResources/ActorMacros.Switch Has Authority`
    (:`Authority`
      (cast `/Game/Blueprint/BP_IceBall` OtherActor)
      (if (`|EnumEquality` (`self.BoundType`) "WinBound")
        (`KismetSystemLibrary.PrintString` (`KismetStringLibrary.Concat_StrStr` "玩家" (`KismetStringLibrary.Conv_IntToString` (`self.PlayerIndex`)) "输了") true true (struct :`G` 0.66 :`B` 1.0 :`A` 1.0) 50.0)))))

(fn `UserConstructionScript`
  (bind _returnvalue (`KismetMaterialLibrary.CreateDynamicMaterialInstance` "/Game/Material/M_Transparent.M_Transparent"))
  (set `self.Material` _returnvalue)
  (`MaterialInstanceDynamic.SetScalarParameterValue` (`self.Material`) "Debug" 1.0)
  (`PrimitiveComponent.SetMaterial` (`self.Plane`) 0 (`self.Material`)))